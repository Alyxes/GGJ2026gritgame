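; AC_Change is a component that records a solved anomaly and reports the new count to the level's door.
; On BeginPlay it caches the MyGameInstance reference.
; IsDone increments the game instance's SolvedAnomalys counter, looks up BP_Door by class and passes the updated count through DoorMessage, with debug prints before and after.
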(event EventBeginPlay
  (bind _asmy_game_instance (Utilities|Casting|CastToMyGameInstance (Game|GetGameInstance)))
  (Variables|Default|SetAs%20My%20Game%20Instance _asmy_game_instance))

(fn IsDone?
  (bind _as_my_game_instance (Variables|Default|GetAs%20My%20Game%20Instance))
  (Development|PrintString "Gay sex")
  (bind _result (Math|Integer|IncrementInt (Variables|/Game/GritGames/Marcus/MyGameInstance.MyGameInstance_C|GetSolvedAnomalys _as_my_game_instance))
    (:%20%20
      (Variables|/Game/GritGames/Marcus/MyGameInstance.MyGameInstance_C|SetSolvedAnomalys _as_my_game_instance _result)
      (bind _returnvalue (Actor|GetActorOfClass "/Game/GritGames/Marcus/BP_Door.BP_Door_C"))
      (Class|BPIDoor|Door(Message) _returnvalue (Variables|/Game/GritGames/Marcus/MyGameInstance.MyGameInstance_C|GetSolvedAnomalys (Variables|Default|GetAs%20My%20Game%20Instance)))
      (Development|PrintString "Gay sex"))))