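; Shadow enemy AI character that is visible, smoking and pawn-blocking only while the game instance's MaskOn flag is set, polled by a looping timer.
; With the mask on, a trigger overlap sets the SeeingPlayer blackboard key; exposed events also set it and switch walk/chase speed.
; AttackPlayer plays a montage, then applies damage through a delayed forward sphere trace.
; Pawn sensing is unused, and the screen-shake trigger only runs a cooldown.
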(event OnSeePawn(PawnSensing)
  (params (Pawn :type Pawn%20Object%20Reference)))

(event OnComponentBeginOverlap(Trigger)
  (params (OverlappedComponent :type Primitive%20Component%20Object%20Reference) (OtherActor :type Actor%20Object%20Reference) (OtherComp :type Primitive%20Component%20Object%20Reference) (OtherBodyIndex :type Integer) (bFromSweep :type Boolean) (SweepResult :type Hit%20Result%20Structure%20%28by%20ref%29))
  ;[0.1421 0 0.15 0.5] ScreenShake
  (if (not (Variables|Default|GetDelayOn))
    (Utilities|Casting|CastToBP_FirstPersonCharacter OtherActor)
    (CallFunction|Delay)))

(event OnComponentBeginOverlap(Trigger2)
  (params (OverlappedComponent :type Primitive%20Component%20Object%20Reference) (OtherActor :type Actor%20Object%20Reference) (OtherComp :type Primitive%20Component%20Object%20Reference) (OtherBodyIndex :type Integer) (bFromSweep :type Boolean) (SweepResult :type Hit%20Result%20Structure%20%28by%20ref%29))
  (if (Variables|/Game/GritGames/Marcus/MyGameInstance.MyGameInstance_C|GetMaskOn (Variables|Default|GetAs%20My%20Game%20Instance))
    (Utilities|Casting|CastToBP_FirstMarcusPerson OtherActor)
    (AI|Components|Blackboard|SetValueasBool (AI|GetBlackboard (AI|GetAIController self)) (Utilities|Name|MakeLiteralName "SeeingPlayer") true)))

(event Custom|AttackPlayer
  (bind _attacktracepoint (Variables|Default|GetAttackTracePoint))
  (bind _returnvalue (Transformation|GetWorldLocation _attacktracepoint))
  (if (not (Variables|Default|GetAttacking?))
    (Variables|Default|SetAttacking? true)
    (Animation|Montage|PlayMontage (Variables|Character|GetMesh) "/Game/GritGames/Marcus/Ai/Anim_Attack_Montage.Anim_Attack_Montage"
      (:then
        (Utilities|FlowControl|Delay (Variables|AttackV|GetAttackSpeed))
        (bind _outhit (Collision|SphereTraceForObjects _returnvalue (+ _returnvalue (* (Math|Vector|GetForwardVector (Transformation|GetWorldRotation _attacktracepoint)) 7e+01)) (Variables|AttackV|GetAttackRange) (Utilities|Array|MakeArray "ObjectTypeQuery3") false 0 "None"))
        (if true
          (Game|Damage|ApplyDamage (.HitActor (Collision|BreakHitResult _outhit)) 1.0 0 0)))
      (:OnCompleted
        (Variables|Default|SetAttacking? false)))))

(event Custom|Stop%20Seeing%20Player
  (AI|Components|Blackboard|SetValueasBool (AI|GetBlackboard (AI|GetAIController self)) (Utilities|Name|MakeLiteralName "SeeingPlayer") false))

(event Custom|ShowThis
  (bind _ns_shadowsmoke (Variables|Default|GetNS_ShadowSmoke))
  (if (Variables|/Game/GritGames/Marcus/MyGameInstance.MyGameInstance_C|GetMaskOn (Variables|Default|GetAs%20My%20Game%20Instance))
    (Rendering|SetVisibility (Variables|Character|GetMesh) true true)
    (Components|Activation|Activate _ns_shadowsmoke false)
    (Collision|SetCollisionResponsetoChannel (Variables|Collision|GetCapsuleComponent) "ECC_Pawn" "ECR_Block")
    (else
      (Rendering|SetVisibility (Variables|Character|GetMesh) false false)
      (Components|Activation|Deactivate _ns_shadowsmoke)
      (Collision|SetCollisionResponsetoChannel (Variables|Collision|GetCapsuleComponent) "ECC_Pawn" "ECR_Ignore"))))

(event Custom|Delay
  ;[0.1421 0 0.15 0.5] ScreenShake
  (Variables|Default|SetDelayOn true)
  (Utilities|FlowControl|Delay 11.0)
  (Variables|Default|SetDelayOn false))

(event Custom|SetWalkingSpeed
  (params (IsChassing? :type Boolean))
  (bind _charactermovement (Variables|Character|GetCharacterMovement))
  (if IsChassing?
    (Variables|/Script/Engine.CharacterMovementComponent|SetMaxWalkSpeed _charactermovement (Variables|Speeds|GetChaaseSpeed))
    (else
      (Variables|/Script/Engine.CharacterMovementComponent|SetMaxWalkSpeed _charactermovement (Variables|Speeds|GetWalkSpeep)))))

(event EventBeginPlay
  (Variables|/Script/Engine.CharacterMovementComponent|SetMaxWalkSpeed (Variables|Character|GetCharacterMovement) (Variables|Speeds|GetWalkSpeep))
  (CallFunction|GetonStart)
  (Utilities|Time|SetTimerbyEvent 0 0.8 true)
  (Utilities|Time|SetTimerbyEvent (delegate Custom|ShowThis) 0.1 true))

(event EventSeeingPlayer
  (params (IsSeeing? :type Boolean))
  (CallFunction|SetWalkingSpeed IsSeeing?)
  (AI|Components|Blackboard|SetValueasBool (AI|GetBlackboard (AI|GetAIController self)) (Utilities|Name|MakeLiteralName "SeeingPlayer") IsSeeing?))

(fn ConstructionScript)

(fn GetonStart
  (bind _asmy_game_instance (Utilities|Casting|CastToMyGameInstance (Game|GetGameInstance)))
  (Variables|Default|SetAs%20My%20Game%20Instance _asmy_game_instance))