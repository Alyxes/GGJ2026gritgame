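; AI character Blueprint, named as a toilet enemy, that on BeginPlay sets its walk speed, caches MyGameInstance and starts two looping timers with no visible handlers.
; Its see-pawn, stop-seeing and attack events are empty.
; Disconnected logic holds a montage-driven sphere-trace melee attack and SeeingPlayer blackboard updates, with sighting gated on the game instance's MaskOn and the Player tag, so none of it runs.
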(event OnSeePawn(PawnSensing)
  (params (Pawn :type Pawn%20Object%20Reference)))

(event Custom|AttackPlayer)

(event Custom|Stop%20Seeing%20Player)

(event EventBeginPlay
  (Variables|/Script/Engine.CharacterMovementComponent|SetMaxWalkSpeed (Variables|Character|GetCharacterMovement) (Variables|Speeds|GetWalkSpeep))
  (CallFunction|GetonStart)
  (Utilities|Time|SetTimerbyEvent 0 0.8 true)
  (Utilities|Time|SetTimerbyEvent 0 0.1 true))

(fn ConstructionScript)

(fn GetonStart
  (bind _asmy_game_instance (Utilities|Casting|CastToMyGameInstance (Game|GetGameInstance)))
  (Variables|Default|SetAs%20My%20Game%20Instance _asmy_game_instance))