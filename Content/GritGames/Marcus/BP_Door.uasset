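; Door actor that opens once by swapping a closed component for one of two pre-placed open variants, with no animation.
; BeginPlay disables collision on both open variants.
; When its OpenAmount comparison passes, the Door event destroys DoorClosed, reveals and enables collision on one variant, and plays a 2D creak.
; The OpenOut flag picks the variant in apparently inverted fashion: true shows DoorOpenIn, false shows DoorOpenOut.
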(event EventBeginPlay
  (Collision|SetCollisionEnabled (Variables|Default|GetDoorOpenIn) "NoCollision")
  (Collision|SetCollisionEnabled (Variables|Default|GetDoorOpenOut) "NoCollision"))

(event EventDoor
  (params (OpenAmount :type Integer))
  (bind _dooropenin (Variables|Default|GetDoorOpenIn))
  (bind _dooropenout (Variables|Default|GetDoorOpenOut))
  (if (== OpenAmount (Variables|Default|GetOpenAmount))
    (Components|DestroyComponent (Variables|Default|GetDoorClosed))
    (if (Variables|Default|GetOpenOut?)
      (Collision|SetCollisionEnabled _dooropenin "QueryAndPhysics")
      (Rendering|SetVisibility _dooropenin true true)
      (else
        (Collision|SetCollisionEnabled _dooropenout "QueryAndPhysics")
        (Rendering|SetVisibility _dooropenout true true)))
    (Audio|PlaySound2D "/Game/GritGames/Matti/GJ2026/Anomalys/Door_Creak.Door_Creak" 1.0 1.0 0.0 0 0)))

(fn ConstructionScript)