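; BP_MovingChair is a chair that starts moving once the first-person character overlaps its trigger box.
; The overlap sets a Loop flag, and Tick then calls MoveComponentTo toward a relative X of MoveAmont, timed by Speed.
; BeginPlay saves the chair's start position and rotation, which nothing shown reads.
; Disconnected spline-placement and wrap-around logic never runs, and Loop is never cleared.
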(event OnComponentBeginOverlap(TriggerBox)
  (params (OverlappedComponent :type Primitive%20Component%20Object%20Reference) (OtherActor :type Actor%20Object%20Reference) (OtherComp :type Primitive%20Component%20Object%20Reference) (OtherBodyIndex :type Integer) (bFromSweep :type Boolean) (SweepResult :type Hit%20Result%20Structure%20%28by%20ref%29))
  (Utilities|Casting|CastToBP_FirstPersonCharacter OtherActor)
  (Variables|Default|SetLoop? true))

(event EventBeginPlay
  (bind _chair (Variables|Default|GetChair))
  (Variables|Default|SetStartPos (Transformation|GetWorldLocation _chair))
  (Variables|Default|SetStartRot (Transformation|GetWorldRotation _chair)))

(event EventTick
  (params (DeltaSeconds :type Float%20%28single-precision%29))
  (if (Variables|Default|GetLoop?)
    (Components|MoveComponentTo (Variables|Default|GetChair) (Math|Vector|MakeVector (Variables|Default|GetmoveAmont) 0.0 0.0) "0, 0, 0" false false (Variables|Default|GetSpeed) false)))

(fn ConstructionScript)