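; Interactable screen anomaly that can be solved while the player's mask is on, unless it is flagged as fake.
; A looping timer polls the mask state and applies the Type behavior: visibility, material swap, or outline and static-screen glow through dynamic materials.
; Interacting plays a sound, increments the GameInstance solved count, sends it to Door-tagged actors, then destroys the screen or turns off its glow.
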(event Custom|ShowThis
  (CallFunction|TypeI (and (Variables|/Game/GritGames/Marcus/MyGameInstance.MyGameInstance_C|GetMaskOn (Variables|Default|GetAs%20My%20Game%20Instance)) (not (Variables|_|GetIsPickedUp?))) (Variables|Default|Getmesh)))

(event EventBeginPlay
  (bind _asmy_game_instance (Utilities|Casting|CastToMyGameInstance (Game|GetGameInstance)))
  (Variables|Default|SetAs%20My%20Game%20Instance _asmy_game_instance)
  (Utilities|Time|SetTimerbyEvent (delegate Custom|ShowThis) 0.1 true)
  (Utilities|FlowControl|Sequence
    (:then_0
      (if (not (Variables|AnomalySettings|GetIsFakeAnomaly))
        (bind _returnvalue (Rendering|Material|CreateDynamicMaterialInstance "/Game/GritGames/William/VFX/MI_InteractiveObject.MI_InteractiveObject" "None" "None" :!class /Script/Engine.KismetMaterialLibrary))
        (bind _output_get (Variables|Default|SetOutlineInstanc _returnvalue))
        (Rendering|Material|SetOverlayMaterial (Variables|Default|Getmesh) _output_get :!class /Script/Engine.MeshComponent)))
    (:then_1
      (bind _returnvalue_2 (Rendering|Material|CreateDynamicMaterialInstance "/Game/GritGames/Zelma/MI_Screen_Static.MI_Screen_Static" "None" "None" :!class /Script/Engine.KismetMaterialLibrary))
      (bind _output_get_2 (Variables|Default|SetStaticScreenInstance _returnvalue_2))
      (Rendering|Material|SetMaterial (Variables|Default|Getmesh) 1 _output_get_2))))

(event EventInteract
  (if (not (Variables|AnomalySettings|GetIsFakeAnomaly))
    (if (and (Variables|/Game/GritGames/Marcus/MyGameInstance.MyGameInstance_C|GetMaskOn (Variables|Default|GetAs%20My%20Game%20Instance)) (not (Variables|_|GetIsPickedUp?)))
      (Variables|_|SetIsPickedUp? true)
      (Audio|PlaySound2D "/Game/GritGames/Marcus/Level/PickUpSound.PickUpSound" 1.0 1.0 0.0 0 0)
      (if (Variables|_|GetSelfDestroy)
        (CallFunction|ChangeDoor)
        (Actor|DestroyActor)
        (else
          (CallFunction|ChangeDoor)
          (Rendering|Material|SetScalarParameterValue (Variables|Default|GetStaticScreenInstance) "EmissiveStrength" 0.0 :!class /Script/Engine.MaterialInstanceDynamic))))))

(fn ConstructionScript)

(fn ChangeDoor
  (bind _as_my_game_instance (Variables|Default|GetAs%20My%20Game%20Instance))
  (bind _result (Math|Integer|IncrementInt (Variables|/Game/GritGames/Marcus/MyGameInstance.MyGameInstance_C|GetSolvedAnomalys _as_my_game_instance))
    (:%20%20
      (Variables|/Game/GritGames/Marcus/MyGameInstance.MyGameInstance_C|SetSolvedAnomalys _as_my_game_instance _result)
      (bind _outactors (Actor|GetAllActorswithTag "Door"))
      (for _array_element _outactors
        (Class|BPIDoor|Door(Message) _array_element (Variables|/Game/GritGames/Marcus/MyGameInstance.MyGameInstance_C|GetSolvedAnomalys (Variables|Default|GetAs%20My%20Game%20Instance)))))))

(fn TypeI
  (params (ISTRUE? :type Boolean) (Object :type Static%20Mesh%20Component%20Object%20Reference))
  (bind _type (Variables|_|GetType))
  (bind _outlineinstanc (Variables|Default|GetOutlineInstanc))
  (Variables|Default|SetObject Object)
  (if ISTRUE?
    (switch Utilities|FlowControl|Switch|SwitchonInteractType _type
      (:NewEnumerator0
        (Rendering|SetVisibility (Variables|Default|GetObject) true true))
      (:NewEnumerator1
        (Rendering|Material|SetMaterial (Variables|Default|GetObject) 0 (Variables|Materials|GetMat_Show)))
      (:NewEnumerator2
        (Utilities|IsValid _outlineinstanc :!label _label
          (:Is%20Valid
            (Rendering|Material|SetScalarParameterValue _outlineinstanc "OutlineVisibilityValue" (Math|Float|SelectFloat 1.0 0.0 ISTRUE?) :!class /Script/Engine.MaterialInstanceDynamic))
          (:Is%20Not%20Valid
            _))
        (Rendering|Material|SetScalarParameterValue (Variables|Default|GetStaticScreenInstance) "EmissiveStrength" (select (Variables|AnomalySettings|GetIsFakeAnomaly) 1.0 (select (Variables|_|GetIsPickedUp?) 0.0 1.0)) :!class /Script/Engine.MaterialInstanceDynamic)))
    (else
      (switch Utilities|FlowControl|Switch|SwitchonInteractType _type
        (:NewEnumerator0
          (Rendering|SetVisibility (Variables|Default|GetObject) false false))
        (:NewEnumerator1
          (Rendering|Material|SetMaterial (Variables|Default|GetObject) 0 (Variables|Materials|GetMat_Hide)))
        (:NewEnumerator2
          (goto _label))))))