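; BP_interactWIN is an interactable object that shows the BP_Win widget when used once while the game instance's mask is on.
; A looping timer feeds the mask and pickup state into TypeI, which toggles visibility, material or an overlay outline according to Type.
; The outline uses a dynamic material instance.
; ChangeDoor increments the solved-anomaly count and messages Door-tagged actors, but nothing here calls it.
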(event Custom|ShowThis
  (CallFunction|TypeI (and (Variables|/Game/GritGames/Marcus/MyGameInstance.MyGameInstance_C|GetMaskOn (Variables|Default|GetAs%20My%20Game%20Instance)) (not (Variables|_|GetIsPickedUp?))) (Variables|Default|Getmesh)))

(event EventBeginPlay
  (bind _asmy_game_instance (Utilities|Casting|CastToMyGameInstance (Game|GetGameInstance)))
  (Variables|Default|SetAs%20My%20Game%20Instance _asmy_game_instance)
  (Utilities|Time|SetTimerbyEvent (delegate Custom|ShowThis) 0.1 true)
  (bind _returnvalue (Rendering|Material|CreateDynamicMaterialInstance "/Game/GritGames/William/VFX/MI_InteractiveObject.MI_InteractiveObject" "None" "None" :!class /Script/Engine.KismetMaterialLibrary))
  (bind _output_get (Variables|Default|SetOutlineInstanc _returnvalue))
  (Rendering|Material|SetOverlayMaterial (Variables|Default|Getmesh) _output_get :!class /Script/Engine.MeshComponent))

(event EventInteract
  (if (and (Variables|/Game/GritGames/Marcus/MyGameInstance.MyGameInstance_C|GetMaskOn (Variables|Default|GetAs%20My%20Game%20Instance)) (not (Variables|_|GetIsPickedUp?)))
    (Variables|_|SetIsPickedUp? true)
    (bind _returnvalue (UserInterface|CreateWidget "/Game/GritGames/Filippa/BP/BP_Win.BP_Win_C" (Game|GetPlayerController 0)))
    (UserInterface|Viewport|AddtoViewport _returnvalue 0)))

(fn ConstructionScript)

(fn ChangeDoor
  (bind _as_my_game_instance (Variables|Default|GetAs%20My%20Game%20Instance))
  (bind _result (Math|Integer|IncrementInt (Variables|/Game/GritGames/Marcus/MyGameInstance.MyGameInstance_C|GetSolvedAnomalys _as_my_game_instance))
    (:%20%20
      (Variables|/Game/GritGames/Marcus/MyGameInstance.MyGameInstance_C|SetSolvedAnomalys _as_my_game_instance _result)
      (bind _outactors (Actor|GetAllActorswithTag "Door"))
      (for _array_element _outactors
        (Class|BPIDoor|Door(Message) _array_element (Variables|/Game/GritGames/Marcus/MyGameInstance.MyGameInstance_C|GetSolvedAnomalys (Variables|Default|GetAs%20My%20Game%20Instance)))))))

(fn TypeI
  (params (ISTRUE? :type Boolean) (Object :type Static%20Mesh%20Component%20Object%20Reference))
  (bind _type (Variables|_|GetType))
  (Variables|Default|SetObject Object)
  (if ISTRUE?
    (switch Utilities|FlowControl|Switch|SwitchonInteractType _type
      (:NewEnumerator0
        (Rendering|SetVisibility (Variables|Default|GetObject) true true))
      (:NewEnumerator1
        (Rendering|Material|SetMaterial (Variables|Default|GetObject) 0 (Variables|Materials|GetMat_Show)))
      (:NewEnumerator2
        (Rendering|Material|SetScalarParameterValue (Variables|Default|GetOutlineInstanc) "OutlineVisibilityValue" (Math|Float|SelectFloat 1.0 0.0 ISTRUE?) :!class /Script/Engine.MaterialInstanceDynamic :!label _label)))
    (else
      (switch Utilities|FlowControl|Switch|SwitchonInteractType _type
        (:NewEnumerator0
          (Rendering|SetVisibility (Variables|Default|GetObject) false false))
        (:NewEnumerator1
          (Rendering|Material|SetMaterial (Variables|Default|GetObject) 0 (Variables|Materials|GetMat_Hide)))
        (:NewEnumerator2
          (goto _label))))))