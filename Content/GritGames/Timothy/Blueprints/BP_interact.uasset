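; Interactable anomaly actor that reveals itself while the player's mask is on, using the MaskOn flag in MyGameInstance.
; A looping timer polls that flag and, depending on Type, toggles the Sphere's visibility or swaps its material.
; Interacting with the mask on prints a debug string and, if SelfDestroy is set, destroys the actor, increments SolvedAnomalys and sends the count to all Door-tagged actors.
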(event Custom|ShowThis
  (CallFunction|TypeI (Variables|/Game/GritGames/Marcus/MyGameInstance.MyGameInstance_C|GetMaskOn (Variables|Default|GetAs%20My%20Game%20Instance)) (Variables|Default|GetSphere)))

(event EventBeginPlay
  (bind _asmy_game_instance (Utilities|Casting|CastToMyGameInstance (Game|GetGameInstance)))
  (Variables|Default|SetAs%20My%20Game%20Instance _asmy_game_instance)
  (Utilities|Time|SetTimerbyEvent (delegate Custom|ShowThis) 0.1 true))

(event EventInteract
  (if (Variables|/Game/GritGames/Marcus/MyGameInstance.MyGameInstance_C|GetMaskOn (Variables|Default|GetAs%20My%20Game%20Instance))
    (Development|PrintString "tettete" true true "(R=0.862374,G=0.000000,B=1.000000,A=1.000000)")
    (if (Variables|_|GetSelfDestroy)
      (Actor|DestroyActor)
      (CallFunction|ChangeDoor))))

(fn ConstructionScript)

(fn ChangeDoor
  (bind _as_my_game_instance (Variables|Default|GetAs%20My%20Game%20Instance))
  (bind _result (Math|Integer|IncrementInt (Variables|/Game/GritGames/Marcus/MyGameInstance.MyGameInstance_C|GetSolvedAnomalys _as_my_game_instance))
    (:%20%20
      (Variables|/Game/GritGames/Marcus/MyGameInstance.MyGameInstance_C|SetSolvedAnomalys _as_my_game_instance _result)
      (bind _outactors (Actor|GetAllActorswithTag "Door"))
      (for _array_element _outactors
        (Class|BPIDoor|Door(Message) _array_element (Variables|/Game/GritGames/Marcus/MyGameInstance.MyGameInstance_C|GetSolvedAnomalys (Variables|Default|GetAs%20My%20Game%20Instance)))))))

(fn TypeI
  (params (ISTRUE? :type Boolean) (Object :type Static%20Mesh%20Component%20Object%20Reference))
  (bind _type (Variables|_|GetType))
  (Variables|Default|SetObject Object)
  (if ISTRUE?
    (switch Utilities|FlowControl|Switch|SwitchonInteractType _type
      (:NewEnumerator0
        (Rendering|SetVisibility (Variables|Default|GetObject) true true))
      (:NewEnumerator1
        (Rendering|Material|SetMaterial (Variables|Default|GetObject) 0 (Variables|Materials|GetMat_Show))))
    (else
      (switch Utilities|FlowControl|Switch|SwitchonInteractType _type
        (:NewEnumerator0
          (Rendering|SetVisibility (Variables|Default|GetObject) false false))
        (:NewEnumerator1
          (Rendering|Material|SetMaterial (Variables|Default|GetObject) 0 (Variables|Materials|GetMat_Hide)))))))