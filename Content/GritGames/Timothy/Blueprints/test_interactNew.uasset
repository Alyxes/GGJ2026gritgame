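; Test interactable actor with a sphere that changes color based on whether the player's mask is on, as stored in the game instance.
; On BeginPlay it caches MyGameInstance and starts a looping timer that polls MaskOn, setting the sphere to the blue material when on and red when off.
; Its Interact event destroys the actor only when the mask is on and SelfDestroy is enabled.
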(event Custom|ShowThis
  ;[0.15 0.15 0.15 0.5] Switching material
  (if (Variables|/Game/GritGames/Marcus/MyGameInstance.MyGameInstance_C|GetMaskOn (Variables|Default|GetAs%20My%20Game%20Instance))
    (Rendering|Material|SetMaterial (Variables|Default|GetSphere) 0 "/Game/GritGames/Timothy/Materials/BlueMaterial.BlueMaterial")
    (else
      (Rendering|Material|SetMaterial (Variables|Default|GetSphere) 0 "/Game/GritGames/Timothy/Materials/RedMaterial.RedMaterial"))))

(event EventBeginPlay
  (bind _asmy_game_instance (Utilities|Casting|CastToMyGameInstance (Game|GetGameInstance)))
  (Variables|Default|SetAs%20My%20Game%20Instance _asmy_game_instance)
  (Utilities|Time|SetTimerbyEvent (delegate Custom|ShowThis) 0.1 true))

(event EventInteract
  ;[0.15 0.15 0.15 0.5] Interacting is destroying
  (if (Variables|/Game/GritGames/Marcus/MyGameInstance.MyGameInstance_C|GetMaskOn (Variables|Default|GetAs%20My%20Game%20Instance))
    (if (Variables|_|GetSelfDestroy)
      (Actor|DestroyActor))))

(fn ConstructionScript)