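; Actor component that toggles a glitch vision post-process effect on its owner.
; On BeginPlay it finds the owner's PostProcessComponent, makes it unbound at zero weight and assigns the glitch material as a weighted blendable.
; OnMaskVisionToggle flip-flops a target weight between on and off.
; Tick copies that target straight to the component's blend weight, so the effect switches without interpolation.
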(event Custom|On%20Mask%20Vision%20Toggle
  ;[0.15 0.15 0.15 0.5] Toggle the glitch effect when the event is called
  (bind _isa (Utilities|FlowControl|FlipFlop)
    (:A
      (bind _output_get (Variables|Default|Set_targetWeight 1.0)))
    (:B
      (bind _output_get_2 (Variables|Default|Set_targetWeight 0.0)))))

(event EventBeginPlay
  ;[0.15 0.15 0.15 0.5] Set up the post processing component based on the owner of this component
  (bind _output_get (Variables|Default|Set_postProcessingComponent (Actor|GetComponentbyClass (Components|GetOwner) "/Script/Engine.PostProcessComponent")))
  (Variables|/Script/Engine.PostProcessComponent|SetbUnbound _output_get true)
  (bind _output_get_2 (Variables|/Script/Engine.PostProcessComponent|SetBlendWeight _output_get 0.0))
  (Variables|Default|Set_currentBlendWeight _output_get_2)
  (Variables|/Script/Engine.PostProcessComponent|SetSettings _output_get (Utilities|Struct|MakePostProcessSettings (Utilities|Struct|MakeWeightedBlendables (Utilities|Array|MakeArray (Utilities|Struct|MakeWeightedBlendable 1.0 (Variables|Default|Get_postProcessingMaterial)))))))

(event EventTick
  (params (DeltaSeconds :type Float%20%28single-precision%29))
  ;[0.15 0.15 0.15 0.5] Toggle the glitch effect when the event is called
  (Variables|/Script/Engine.PostProcessComponent|SetBlendWeight (Variables|Default|Get_postProcessingComponent) (select (stale Custom|On%20Mask%20Vision%20Toggle _isa) (stale Custom|On%20Mask%20Vision%20Toggle _output_get_2) (stale Custom|On%20Mask%20Vision%20Toggle _output_get))))